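; Rifle weapon actor that attaches its mesh to the player's third-person character when play begins.
; BeginPlay runs the parent logic, casts player pawn 0 to BP_ThirdPersonCharacter, then attaches WeaponMesh to the Rifle_Socket on the character mesh with relative transform rules and prints a debug message.
; It has no firing or pickup logic of its own; overlap and tick events are disabled, and construction only calls the parent.
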(event `self.ReceiveBeginPlay`
  (`parent.ReceiveBeginPlay`)
  (bind _asbp_third_person_character (cast `/Game/ThirdPerson/Blueprints/BP_ThirdPersonCharacter` (`GameplayStatics.GetPlayerPawn` 0)))
  (`SceneComponent.K2_AttachToComponent` (`self.Weapon_Mesh`) (`Character.Mesh` _asbp_third_person_character) "Rifle_Socket" "KeepRelative" "KeepRelative" "KeepRelative" true)
  (`KismetSystemLibrary.PrintString` "Attached Rifle"))

(fn `UserConstructionScript`
  (`parent.UserConstructionScript`))