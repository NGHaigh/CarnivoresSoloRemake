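; Base weapon actor that configures itself from a row in a weapon data table.
; On BeginPlay it looks up its row name, stores the row as WeaponData, applies that row's skeletal mesh and prints the weapon type.
; GetWeaponData exposes the stored row.
; FIreWeapon is a placeholder with a constant condition, so it only prints "Out of Ammo" and never reaches the "Fired" message.
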(event `self.ReceiveBeginPlay`
  (bind _returnvalue (`|GetDataTableRow` (`self.WeaponDataTable`) (`self.WeaponRowName`))
    (:`then`
      (bind _output_get (set `self.WeaponData` _returnvalue))
      (`KismetSystemLibrary.PrintString` (`|GetEnumeratorNameAsString` (break `/Game/Weapon_System/Data_Structs/Weapon_Data` _output_get)))
      (`SkeletalMeshComponent.SetSkeletalMeshAsset` (`self.Weapon_Mesh`) (`.Mesh_5_245EF98E4B6C0EE4307D969BADEE5F2E` (break `/Game/Weapon_System/Data_Structs/Weapon_Data` _output_get))))
    (:`RowNotFound`
      (`KismetSystemLibrary.PrintString` "Failed"))))

(fn `FIreWeapon`
  (if true
    (`KismetSystemLibrary.PrintString` "Out of Ammo")))

(fn `GetWeaponData`
  (returns (WeaponData :type "/Game/Weapon_System/Data_Structs/Weapon_Data Structure"))
  (return (`self.WeaponData`)))

(fn `UserConstructionScript`)